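; BP_cableActor builds a row of static meshes along a spline with sagging cables strung between them, like poles and wires, in the construction script.
; A boolean picks placement at each spline point or at even intervals from mesh length plus spacing.
; Each cable starts and ends at a height offset, its length scaled by span distance.
; Point mode creates a separate instanced mesh component per point; interval mode shares one.
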(fn `CablesByPoints`
  (bind (_returnvalue_inputkey _returnvalue_position) (break `SplinePoint` (`SplineComponent.GetSplinePointAt` (`self.Spline`) (`self.PointIndex`) "Local")))
  (bind _returnvalue (`SplineComponent.GetTransformAtSplinePoint` (`self.Spline`) (`self.PointIndex`) "Local" false))
  (bind (_returnvalue_inputkey_2 _returnvalue_position_2) (break `SplinePoint` (`SplineComponent.GetSplinePointAt` (`self.Spline`) (+ (`self.PointIndex`) 1) "Local")))
  (for _index (range (+ (- (`SplineComponent.GetNumberOfSplinePoints` (`self.Spline`)) 2) 1))
    (set `self.PointIndex` _index)
    (`|ExecutionSequence`
      (:`then_0`
        ; crea el componente
        (bind _returnvalue_2 (`AddComponent|NODE_AddInstancedStaticMeshComponent-0` :!label _label))
        (set `self.ISMC` _returnvalue_2)
        ; dale una mesh al componente
        (`StaticMeshComponent.SetStaticMesh` (`self.ISMC`) (`self.SM`))
        ; Colocamos instancias en funcion del index
        (`InstancedStaticMeshComponent.AddInstance` (`self.ISMC`) (`KismetMathLibrary.MakeTransform` (.location _returnvalue) (`KismetMathLibrary.MakeRotator` 0.0 0.0 (.yaw (.rotation _returnvalue))) (.scale _returnvalue)) false))
      (:`then_1`
        (bind _returnvalue_3 (`AddComponent|NODE_AddCableComponent-0` :`RelativeTransform` (`KismetMathLibrary.MakeTransform` (`self.CabeZOffset` _returnvalue_position))))
        (set `self.Cable component` _returnvalue_3)
        (set `CableComponent.EndLocation` (`self.CabeZOffset` _returnvalue_position_2) (`self.Cable component`))
        ; Cable length independent distance
        (set `CableComponent.CableLength` (* (`self.CableLength`) (`self.DistanceBetweenSplinePoints` (`self.PointIndex`) (`self.Spline`))) (`self.Cable component`))
        (set `CableComponent.CableWidth` (`self.CableWidth`) (`self.Cable component`)))))
  (`/Engine/EditorBlueprintResources/StandardMacros.IncrementInt` (`self.PointIndex`)
    (:`  `
      (goto _label))))

(fn `CablesByTotalLenght`
  (locals (MeshIndex :type Integer))
  (bind _returnvalue (`SplineComponent.GetLocationAtDistanceAlongSpline` (`self.Spline`) (* (`local.MeshIndex`) (`self.TotalSpacing`)) "Local"))
  (bind _returnvalue_2 (`SplineComponent.GetTransformAtDistanceAlongSpline` (`self.Spline`) (* (`local.MeshIndex`) (`self.TotalSpacing`)) "Local" false))
  (bind _returnvalue_3 (`SplineComponent.GetLocationAtDistanceAlongSpline` (`self.Spline`) (* (+ (`local.MeshIndex`) 1) (`self.TotalSpacing`)) "Local"))
  (bind _sm (`self.SM`)
    (:`then`
      (`|ExecutionSequence`
        (:`then_0`
          (bind (_returnvalue_min _returnvalue_max) (break `Box` (`StaticMesh.GetBoundingBox` _sm)))
          (bind (_returnvalue_x _returnvalue_y _returnvalue_z) (`KismetMathLibrary.BreakVector` (- _returnvalue_max _returnvalue_min)))
          (set `self.MeshLength` _returnvalue_x)
          (set `self.MeshHeight` (* _returnvalue_z (`self.MeshScaleZ`)))
          (bind _returnvalue_4 (`AddComponent|NODE_AddInstancedStaticMeshComponent-1`))
          (bind _output_get (set `self.ISMC` _returnvalue_4))
          (`StaticMeshComponent.SetStaticMesh` _output_get (`self.SM`)))
        (:`then_1`
          (if true
            (bind _output_get_2 (set `self.TotalSpacing` (+ (`self.MeshSpacing`) (`self.MeshLength`))))
            (bind _output_get_3 (set `self.Number meshes` (`KismetMathLibrary.FTrunc` (/ (`SplineComponent.GetSplineLength` (`self.Spline`)) _output_get_2))))
            (for _index (range (+ _output_get_3 1))
              (set `local.MeshIndex` _index)
              (`|ExecutionSequence`
                (:`then_0`
                  (`InstancedStaticMeshComponent.AddInstance` (`self.ISMC`) (`KismetMathLibrary.MakeTransform` (.location _returnvalue_2) (struct) (`KismetMathLibrary.MakeVector` (.x (.scale _returnvalue_2)) (.y (.scale _returnvalue_2)) (* (`self.MeshScaleZ`) (.z (.scale _returnvalue_2))))) false))
                (:`then_1`
                  (if true
                    (bind _returnvalue_5 (`AddComponent|NODE_AddCableComponent-1` :`RelativeTransform` (`KismetMathLibrary.MakeTransform` (`self.CabeZOffset` _returnvalue))))
                    (bind _output_get_4 (set `self.Cable component` _returnvalue_5))
                    (set `CableComponent.EndLocation` (`self.CabeZOffset` _returnvalue_3) _output_get_4)
                    (set `CableComponent.CableLength` (* (`self.CableLength`) (`KismetMathLibrary.Vector_Distance` _returnvalue _returnvalue_3)) (`self.Cable component`))))))))))
    (:`else`)))

(fn `UserConstructionScript`
  (if (`self.ByPoints/ByTotalLenght`)
    (`self.CablesByPoints`)
    (else
      (`self.CablesByTotalLenght`))))