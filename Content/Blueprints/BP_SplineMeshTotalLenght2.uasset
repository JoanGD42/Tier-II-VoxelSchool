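; Construction-script Blueprint that fills a spline with spline mesh components, one for each whole MeshLenght of the spline's total length.
; Each loop pass stores the index and new component, sets X as forward axis and attaches it to the spline with relative transforms.
; The graph sets no start or end positions or tangents on the segments, and the event graph holds only disabled stubs.
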(fn `UserConstructionScript`
  (locals (MeshIndex :type Integer))
  (bind _returnvalue (`KismetMathLibrary.FTrunc` (/ (`SplineComponent.GetSplineLength` (`self.Spline`)) (`self.MeshLenght`))))
  (if (> _returnvalue 0)
    (for _index (range _returnvalue)
      (set `local.MeshIndex` _index)
      (bind _returnvalue_2 (`AddComponent|`))
      (set `self.MeshComponent` _returnvalue_2)
      (`SplineMeshComponent.SetForwardAxis` "X")
      (`SceneComponent.K2_AttachToComponent` (`self.Spline`) "None" "KeepRelative" "KeepRelative" "KeepRelative"))))