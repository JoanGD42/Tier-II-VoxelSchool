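; PCG Blueprint actor that exposes base mesh, over mesh and scatter settings to a PCG graph, apparently for foliage over meshes.
; The construction script calls Cleanup and Generate on the PCG component, then Parameters writes meshes, direction, size and density as named graph parameters.
; Parameters are set after the Generate call, and the FoliageDensity setter has no graph instance connected.
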(event EventBeginPlay)

(event Collision|EventActorBeginOverlap
  (params (OtherActor :type Actor%20Object%20Reference)))

(event EventTick
  (params (DeltaSeconds :type Float%20%28single-precision%29)))

(fn ConstructionScript
  (CallFunction|Cleanup)
  (CallFunction|Generate)
  (CallFunction|Parameters))

(fn Cleanup
  (Class|PCGComponent|Cleanup (Variables|Default|GetPCG) false))

(fn Generate
  (PCG|Generate (Variables|Default|GetPCG) false))

(fn Parameters
  (bind _pcg (Variables|Default|GetPCG))
  (bind _graphinstance (Variables|/Script/PCG.PCGComponent|GetGraphInstance _pcg))
  (Audio|Parameter|SetObjectParameter _graphinstance "BaseMesh" (Variables|Default|GetBaseMesh))
  (Audio|Parameter|SetObjectParameter _graphinstance "OverMesh" (Variables|Default|GetOverMesh))
  (Effects|Components|ParticleSystem|SetVectorParameter _graphinstance "FoliageDirection" (Variables|Default|GetScatterMeshDirection))
  (Effects|Components|ParticleSystem|SetFloatParameter _graphinstance "Size" (Variables|Default|GetSize))
  (Effects|Components|ParticleSystem|SetFloatParameter 0 "FoliageDensity" (Variables|Default|GetFoliageDensity)))