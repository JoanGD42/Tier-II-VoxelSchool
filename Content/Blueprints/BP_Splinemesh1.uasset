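; Spline mesh Blueprint that builds a deformed mesh along an editable, optionally closed spline in the construction script.
; CreateSplineMesh adds one spline mesh component per segment, matching point tangents, scale and roll.
; Each segment's GradientStart and GradientEnd material parameters receive normalized spline distance, flippable by a flag, for a gradient spanning the whole length.
; EndCaps then places a single static mesh at the last point, aligned to its arrive tangent plus a rotation offset.
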(fn `CreateSplineMesh`
  (locals (PointIndex :type Integer) (SplineMeshComponent :type "SplineMeshComponent Object Reference"))
  (bind _spline (`self.Spline`))
  (bind _splinemeshcomponent (`local.SplineMeshComponent`))
  (bind _closedloop (`self.ClosedLoop`))
  (bind _splinemeshcomponent_2 (`local.SplineMeshComponent`))
  (bind _pointindex (`local.PointIndex`))
  (bind _spline_2 (`self.Spline`))
  (bind _sm_scale (`self.SM_Scale`))
  (bind _sm_scale_2 (`self.SM_Scale`))
  (bind _splinemeshcomponent_3 (`local.SplineMeshComponent`))
  (bind _spline_3 (`self.Spline`))
  (bind _spline_4 (`self.Spline`))
  (bind _spline_5 (`self.Spline`))
  (bind _pointindex_2 (`local.PointIndex`))
  (bind _returnvalue (`SplineComponent.GetNumberOfSplinePoints` _spline))
  (bind (_returnvalue_x _returnvalue_y _returnvalue_z) (`KismetMathLibrary.BreakVector` (`SplineComponent.GetScaleAtSplinePoint` _spline_2 _pointindex_2)))
  (bind _returnvalue_roll (`KismetMathLibrary.BreakRotator` (`SplineComponent.GetRotationAtSplinePoint` (`self.Spline`) (`local.PointIndex`) "Local")))
  (bind (_location _tangent) (`SplineComponent.GetLocationAndTangentAtSplinePoint` _spline_5 _pointindex "Local"))
  (bind (_returnvalue_x_2 _returnvalue_y_2 _returnvalue_z_2) (`KismetMathLibrary.BreakVector` (`SplineComponent.GetScaleAtSplinePoint` _spline_2 (+ _pointindex_2 1))))
  (bind _returnvalue_roll_2 (`KismetMathLibrary.BreakRotator` (`SplineComponent.GetRotationAtSplinePoint` (`self.Spline`) (+ (`local.PointIndex`) 1) "Local")))
  (bind (_location_2 _tangent_2) (`SplineComponent.GetLocationAndTangentAtSplinePoint` _spline_5 (+ _pointindex 1) "Local"))
  (bind _returnvalue_2 (/ (`SplineComponent.GetDistanceAlongSplineAtSplinePoint` _spline_3 (`local.PointIndex`)) (`SplineComponent.GetSplineLength` _spline_3)))
  (bind _returnvalue_3 (/ (`SplineComponent.GetDistanceAlongSplineAtSplinePoint` _spline_4 (+ (`local.PointIndex`) 1)) (`SplineComponent.GetSplineLength` _spline_4)))
  (`SplineComponent.SetOverrideConstructionScript` _spline false)
  (`SplineComponent.SetClosedLoop` _spline _closedloop true)
  (for _index (range (+ (`KismetMathLibrary.SelectInt` (- _returnvalue 1) (- _returnvalue 2) _closedloop) 1))
    (set `local.PointIndex` _index)
    (bind _returnvalue_4 (`AddComponent|NODE_AddSplineMeshComponent-0`))
    (set `local.SplineMeshComponent` _returnvalue_4)
    (`StaticMeshComponent.SetStaticMesh` _splinemeshcomponent (`self.StaticMesh`))
    (`PrimitiveComponent.SetMaterial` _splinemeshcomponent 0 (`self.SM_Material`))
    (`SplineMeshComponent.SetForwardAxis` (`local.SplineMeshComponent`) (`self.In Forward Axis`) true)
    (`KismetArrayLibrary.Array_Set` (`self.SplineMeshArray`) (`local.PointIndex`) (`local.SplineMeshComponent`))
    (`SceneComponent.K2_AttachToComponent` (`local.SplineMeshComponent`) (`self.Spline`) "None" "KeepRelative" "KeepRelative" "KeepRelative" true)
    (`SplineMeshComponent.SetStartAndEnd` (`local.SplineMeshComponent`) _location _tangent _location_2 _tangent_2 true)
    (`SplineMeshComponent.SetStartScale` _splinemeshcomponent_2 (`KismetMathLibrary.MakeVector2D` (* _sm_scale_2 _returnvalue_y) (* _sm_scale_2 _returnvalue_z)) true)
    (`SplineMeshComponent.SetEndScale` _splinemeshcomponent_2 (`KismetMathLibrary.MakeVector2D` (* _sm_scale _returnvalue_y_2) (* _sm_scale _returnvalue_z_2)) true)
    (`SplineMeshComponent.SetStartRollDegrees` _splinemeshcomponent_3 _returnvalue_roll true)
    (`SplineMeshComponent.SetEndRollDegrees` _splinemeshcomponent_3 _returnvalue_roll_2 true)
    (`MeshComponent.SetScalarParameterValueOnMaterials` (`local.SplineMeshComponent`) "GradientStart" (`KismetMathLibrary.SelectFloat` _returnvalue_2 (- 1.0 _returnvalue_2) (`self.InvertMaterialGradient`)))
    (`MeshComponent.SetScalarParameterValueOnMaterials` (`local.SplineMeshComponent`) "GradientEnd" (`KismetMathLibrary.SelectFloat` _returnvalue_3 (- 1.0 _returnvalue_3) (`self.InvertMaterialGradient`)))))

(fn `EndCaps`
  (locals (SM_ComponentStart :type "StaticMeshComponent Object Reference"))
  (bind _spline (`self.Spline`))
  (bind _sm_componentstart (`local.SM_ComponentStart`))
  (bind _sm_componentstart_2 (`local.SM_ComponentStart`))
  (bind (_returnvalue_inputkey _returnvalue_position _returnvalue_arrivetangent) (break `SplinePoint` (`SplineComponent.GetSplinePointAt` _spline (- (`SplineComponent.GetNumberOfSplinePoints` _spline) 1) "Local")))
  (bind _returnvalue (`AddComponent|NODE_AddStaticMeshComponent-0`))
  (bind _output_get (set `local.SM_ComponentStart` _returnvalue))
  (`StaticMeshComponent.SetStaticMesh` _output_get (`self.EndMesh`))
  (`PrimitiveComponent.SetMaterial` _sm_componentstart_2 0 (`self.Material`))
  (`SceneComponent.K2_AttachToComponent` _sm_componentstart_2 (`self.Spline`) "None" "KeepRelative" "KeepRelative" "KeepRelative" true)
  (`SceneComponent.K2_SetRelativeLocation` _sm_componentstart _returnvalue_position false false)
  (`SceneComponent.K2_SetRelativeRotation` _sm_componentstart (`KismetMathLibrary.ComposeRotators` (`KismetMathLibrary.Conv_VectorToRotator` _returnvalue_arrivetangent) (`self.SM_EndRotation`)) false false))

(fn `UserConstructionScript`
  (`self.CreateSplineMesh`)
  (`self.EndCaps`))