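; Spline-based road actor that builds a track with side walls and a finish line.
; MakeRoad divides the spline into stretched segments, adding spline meshes with cycling road meshes and walls offset by half the road width, all following spline tangents and roll.
; SetFinishLine places a mesh at a fractional distance along the spline with a height offset.
; The construction script runs only SetFinishLine; its MakeRoad call is disconnected.
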(fn `MakeRoad`
  (locals (TrackIndex :type Integer) (SplineMeshComp :type "SplineMeshComponent Object Reference") (WallSide :type Integer) (WallSMC :type "SplineMeshComponent Object Reference"))
  (bind _startandendrotation (`self.StartAndEndRotation`))
  (bind _startandendsplineposandtangent (`self.StartAndEndSplinePosAndTangent`))
  (bind (_road_originalsize_x _road_originalsize_y) (`KismetMathLibrary.BreakVector` (`self.Road_OriginalSize`)))
  (bind _spline (`self.Spline`))
  (bind _trackindex (`local.TrackIndex`))
  (bind _trackindex_2 (`local.TrackIndex`))
  (bind _road_strechedmeshforward (`self.Road_StrechedMeshForward`))
  (bind _scale (`self.Scale`))
  (bind _road_originalsize_x_2 (`KismetMathLibrary.BreakVector` (`self.Road_OriginalSize`)))
  (bind _road_originalsize_x_3 (`KismetMathLibrary.BreakVector` (`self.Road_OriginalSize`)))
  (bind _splinemeshcomp (`local.SplineMeshComp`))
  (bind _road_strechedmeshforward_2 (`self.Road_StrechedMeshForward`))
  (bind _trackindex_3 (`local.TrackIndex`))
  (bind _spline_2 (`self.Spline`))
  (bind _spline_3 (`self.Spline`))
  (bind _road_strechedmeshforward_3 (`self.Road_StrechedMeshForward`))
  (bind _wallsmc (`local.WallSMC`))
  (bind _wallsmc_2 (`local.WallSMC`))
  (bind _returnvalue (`KismetMathLibrary.Conv_DoubleToVector2D` (`self.Wall_Scale`)))
  (bind _returnvalue_2 (`KismetMathLibrary.Conv_DoubleToVector2D` (`self.Scale`)))
  (bind (_location _tangent) (`self.FitSplineMeshAlongSpline` _spline_2 _trackindex_2 _road_strechedmeshforward_3))
  (bind _returnvalue_3 (/ _road_originalsize_y 2.0))
  (bind (_returnvalue_min _returnvalue_max) (break `Box` (`StaticMesh.GetBoundingBox` (`|GetArrayItem` (`self.SM_RoadArray`)))))
  (bind _returnvalue_roll (`KismetMathLibrary.BreakRotator` (`SplineComponent.GetRotationAtDistanceAlongSpline` _spline_3 (* _trackindex_3 _road_strechedmeshforward_2) "Local")))
  (bind (_location_2 _tangent_2) (`self.FitSplineMeshAlongSpline` _spline_2 (+ _trackindex_2 1) _road_strechedmeshforward_3))
  (bind _returnvalue_roll_2 (`KismetMathLibrary.BreakRotator` (`SplineComponent.GetRotationAtDistanceAlongSpline` _spline_3 (* (+ _trackindex_3 1) _road_strechedmeshforward_2) "Local")))
  (bind _returnvalue_4 (select `int` (`local.WallSide`) :`0` (* _returnvalue_3 -1.0) :`1` _returnvalue_3))
  ; Mesh sizes
  (set `self.Road_OriginalSize` (- (* _returnvalue_max _scale) (* _returnvalue_min _scale)))
  ; Times for the for Loop
  (bind _output_get (set `self.SplineLenght` (`SplineComponent.GetSplineLength` (`self.Spline`))))
  (set `self.NumOfTracks` (`KismetMathLibrary.FFloor` (/ _output_get _road_originalsize_x_3)))
  ; Rescale mesh size to fit into spline
  (if (> (`self.NumOfTracks`) 0)
    (bind _output_get_2 (set `self.Road_StrechedMeshForward` (/ (`self.SplineLenght`) (`self.NumOfTracks`))))
    (if (< (* _road_originalsize_x_2 1.5) _output_get_2)
      (bind _output_get_3 (set `self.NumOfTracks` (+ (`self.NumOfTracks`) 1) :!label _label))
      (set `self.Road_StrechedMeshForward` (/ (`self.SplineLenght`) _output_get_3)))
    (else
      (goto _label)))
  (for _index (range (`self.NumOfTracks`))
    (set `local.TrackIndex` _index)
    (`|ExecutionSequence`
      (:`then_0`
        ; Road For
        ;; Crear SplineMeshComponent
        (bind _returnvalue_5 (`AddComponent|NODE_AddSplineMeshComponent-0`))
        (set `local.SplineMeshComp` _returnvalue_5)
        ;; Get road type
        (`StaticMeshComponent.SetStaticMesh` (`local.SplineMeshComp`) (`|GetArrayItem` (`self.SM_RoadArray`) (select `int` (mod (/ (`local.TrackIndex`) (`self.RoadTypeTimesRepeated`)) (`KismetArrayLibrary.Array_Length` (`self.SM_RoadArray`))) :`0` 0 :`1` 1 :`2` 2)))
        ;; Simple adjusments
        (`SplineMeshComponent.SetForwardAxis` (`local.SplineMeshComp`) (`self.MeshesForwardAxis`) true)
        (`SplineMeshComponent.SetStartScale` _splinemeshcomp _returnvalue_2 true)
        (`SplineMeshComponent.SetEndScale` _splinemeshcomp _returnvalue_2 true)
        (`PrimitiveComponent.SetMaterial` (`local.SplineMeshComp`) 0 (`self.Road_Material`))
        ;; Set start and end position and tangent
        (bind _output_get_4 (set `self.StartAndEndSplinePosAndTangent` (`|MakeArray` _location _tangent _location_2 _tangent_2)))
        (`SplineMeshComponent.SetStartAndEnd` (`local.SplineMeshComp`) (`|GetArrayItem` _output_get_4) (`|GetArrayItem` _output_get_4 1) (`|GetArrayItem` _output_get_4 2) (`|GetArrayItem` _output_get_4 3) true)
        ;; Rotate road
        (bind _output_get_5 (set `self.StartAndEndRotation` (`|MakeArray` _returnvalue_roll _returnvalue_roll_2 :!type "Float (double-precision)")))
        (`SplineMeshComponent.SetStartRollDegrees` (`local.SplineMeshComp`) (`|GetArrayItem` _output_get_5) true)
        (`SplineMeshComponent.SetEndRollDegrees` (`local.SplineMeshComp`) (`|GetArrayItem` _output_get_5 1) true)
        ;; Collisions
        (`PrimitiveComponent.SetCollisionObjectType` (`local.SplineMeshComp`) (`self.CollisionType`))
        (`PrimitiveComponent.SetCollisionEnabled` (`local.SplineMeshComp`) (`self.CollisionEnable`)))
      (:`then_1`
        ; Walls For
        (for _index_2 (range 2)
          (set `local.WallSide` _index_2)
          ;; Crear SplineMeshComponent
          (bind _returnvalue_6 (`AddComponent|NODE_AddSplineMeshComponent-4`))
          (set `local.WallSMC` _returnvalue_6)
          ;; Get mesh
          (`StaticMeshComponent.SetStaticMesh` (`local.WallSMC`) (`self.Walls_Mesh`))
          ;; Simple adjustments
          (`SplineMeshComponent.SetForwardAxis` (`local.WallSMC`) (`self.MeshesForwardAxis`) true)
          (`SplineMeshComponent.SetStartScale` _wallsmc _returnvalue true)
          (`SplineMeshComponent.SetEndScale` _wallsmc _returnvalue true)
          (`PrimitiveComponent.SetMaterial` (`local.WallSMC`) 0 (`self.Wall_Material`))
          ;; Set start and end position and tangent
          (`SplineMeshComponent.SetStartAndEnd` (`local.WallSMC`) (+ (* (`SplineComponent.GetRightVectorAtDistanceAlongSpline` _spline (* _trackindex _road_strechedmeshforward) "Local") _returnvalue_4) (`|GetArrayItem` _startandendsplineposandtangent)) (`|GetArrayItem` _startandendsplineposandtangent 1) (+ (* (`SplineComponent.GetRightVectorAtDistanceAlongSpline` _spline (* (+ _trackindex 1) _road_strechedmeshforward) "Local") _returnvalue_4) (`|GetArrayItem` _startandendsplineposandtangent 2)) (`|GetArrayItem` _startandendsplineposandtangent 3) true)
          ;; Rotate
          (`SplineMeshComponent.SetStartRollDegrees` _wallsmc_2 (`|GetArrayItem` _startandendrotation) true)
          (`SplineMeshComponent.SetEndRollDegrees` _wallsmc_2 (`|GetArrayItem` _startandendrotation 1) true)
          ;; Collisions
          (`PrimitiveComponent.SetCollisionObjectType` (`local.WallSMC`) (`self.CollisionType`))
          (`PrimitiveComponent.SetCollisionEnabled` (`local.WallSMC`) (`self.CollisionEnable`)))))))

(fn `SetFinishLine`
  (locals (SM_Component :type "StaticMeshComponent Object Reference"))
  (bind (_position _rotation) (`self.GetLocationAndRotationAlongSpline` (`self.Spline`) (`self.FL_Location`) (`self.FL_Height`)))
  ; Set Basics
  (bind _returnvalue (`AddComponent|NODE_AddStaticMeshComponent-0`))
  (bind _output_get (set `local.SM_Component` _returnvalue))
  (`StaticMeshComponent.SetStaticMesh` _output_get (`self.FinishLine_SM`))
  (`PrimitiveComponent.SetMaterial` _output_get 0 (`self.FL_Material`))
  ; locate
  (`SceneComponent.K2_SetRelativeLocation` _output_get _position false false)
  (`SceneComponent.K2_SetRelativeRotation` _output_get _rotation false false)
  ; scale
  (`SceneComponent.SetRelativeScale3D` _output_get (`KismetMathLibrary.Conv_DoubleToVector` (`self.FL_Scale`))))

(fn `UserConstructionScript`
  (`self.SetFinishLine`))