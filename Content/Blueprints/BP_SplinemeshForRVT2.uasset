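; Spline mesh actor, named for runtime virtual texture use, that lays a configurable static mesh and material along an editable spline.
; Its construction script adds one spline mesh component per segment, attaches it to the spline and stores it in an array.
; Each segment takes location, tangent, roll and Y/Z scale from its two spline points, with scale multiplied by a shared factor.
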(fn `CreateSplineMesh`
  (locals (PointIndex :type Integer) (SplineMeshComponent :type "SplineMeshComponent Object Reference"))
  (bind _splinemeshcomponent (`local.SplineMeshComponent`))
  (bind _splinemeshcomponent_2 (`local.SplineMeshComponent`))
  (bind _pointindex (`local.PointIndex`))
  (bind _spline (`self.Spline`))
  (bind _sm_scale (`self.SM_Scale`))
  (bind _sm_scale_2 (`self.SM_Scale`))
  (bind _splinemeshcomponent_3 (`local.SplineMeshComponent`))
  (bind _spline_2 (`self.Spline`))
  (bind _pointindex_2 (`local.PointIndex`))
  (bind (_returnvalue_x _returnvalue_y _returnvalue_z) (`KismetMathLibrary.BreakVector` (`SplineComponent.GetScaleAtSplinePoint` _spline _pointindex_2)))
  (bind _returnvalue_roll (`KismetMathLibrary.BreakRotator` (`SplineComponent.GetRotationAtSplinePoint` (`self.Spline`) (`local.PointIndex`) "Local")))
  (bind (_location _tangent) (`SplineComponent.GetLocationAndTangentAtSplinePoint` _spline_2 _pointindex "Local"))
  (bind (_returnvalue_x_2 _returnvalue_y_2 _returnvalue_z_2) (`KismetMathLibrary.BreakVector` (`SplineComponent.GetScaleAtSplinePoint` _spline (+ _pointindex_2 1))))
  (bind _returnvalue_roll_2 (`KismetMathLibrary.BreakRotator` (`SplineComponent.GetRotationAtSplinePoint` (`self.Spline`) (+ (`local.PointIndex`) 1) "Local")))
  (bind (_location_2 _tangent_2) (`SplineComponent.GetLocationAndTangentAtSplinePoint` _spline_2 (+ _pointindex 1) "Local"))
  (for _index (range (+ (- (`SplineComponent.GetNumberOfSplinePoints` (`self.Spline`)) 2) 1))
    (set `local.PointIndex` _index)
    (bind _returnvalue (`AddComponent|NODE_AddSplineMeshComponent-0`))
    (set `local.SplineMeshComponent` _returnvalue)
    (`StaticMeshComponent.SetStaticMesh` _splinemeshcomponent (`self.StaticMesh`))
    (`PrimitiveComponent.SetMaterial` _splinemeshcomponent 0 (`self.SM_Material`))
    (`SplineMeshComponent.SetForwardAxis` (`local.SplineMeshComponent`) (`self.In Forward Axis`) true)
    (`KismetArrayLibrary.Array_Set` (`self.SplineMeshArray`) (`local.PointIndex`) (`local.SplineMeshComponent`))
    (`SceneComponent.K2_AttachToComponent` (`local.SplineMeshComponent`) (`self.Spline`) "None" "KeepRelative" "KeepRelative" "KeepRelative" true)
    (`SplineMeshComponent.SetStartAndEnd` (`local.SplineMeshComponent`) _location _tangent _location_2 _tangent_2 true)
    (`SplineMeshComponent.SetStartScale` _splinemeshcomponent_2 (`KismetMathLibrary.MakeVector2D` (* _sm_scale_2 _returnvalue_y) (* _sm_scale_2 _returnvalue_z)) true)
    (`SplineMeshComponent.SetEndScale` _splinemeshcomponent_2 (`KismetMathLibrary.MakeVector2D` (* _sm_scale _returnvalue_y_2) (* _sm_scale _returnvalue_z_2)) true)
    (`SplineMeshComponent.SetStartRollDegrees` _splinemeshcomponent_3 _returnvalue_roll true)
    (`SplineMeshComponent.SetEndRollDegrees` _splinemeshcomponent_3 _returnvalue_roll_2 true)))

(fn `UserConstructionScript`
  (`self.CreateSplineMesh`))