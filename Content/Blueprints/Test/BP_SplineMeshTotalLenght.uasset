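; Test Blueprint that tiles spline mesh components along the length of its spline.
; The construction script divides the total spline length by a mesh length and truncates the result, so any final partial segment stays uncovered.
; Each segment attaches to the spline with X as forward axis, taking local start and end positions and tangents sampled by distance.
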(fn `UserConstructionScript`
  (locals (MeshIndex :type Integer))
  (bind _spline (`self.Spline`))
  (bind _spline_2 (`self.Spline`))
  (bind _returnvalue (* (`local.MeshIndex`) (`self.MeshLenght`)))
  (bind _returnvalue_2 (* (+ (`local.MeshIndex`) 1) (`self.MeshLenght`)))
  (bind _returnvalue_3 (`KismetMathLibrary.FTrunc` (/ (`SplineComponent.GetSplineLength` (`self.Spline`)) (`self.MeshLenght`))))
  (if (> _returnvalue_3 0)
    (for _index (range _returnvalue_3)
      (set `local.MeshIndex` _index)
      (bind _returnvalue_4 (`AddComponent|NODE_AddSplineMeshComponent-0`))
      (bind _output_get (set `self.SplineMeshComponent` _returnvalue_4))
      (`SplineMeshComponent.SetForwardAxis` _output_get "X" true)
      (`SceneComponent.K2_AttachToComponent` (`self.SplineMeshComponent`) (`self.Spline`) "None" "KeepRelative" "KeepRelative" "KeepRelative" true)
      (`SplineMeshComponent.SetStartAndEnd` (`self.SplineMeshComponent`) (`SplineComponent.GetLocationAtDistanceAlongSpline` _spline_2 _returnvalue "Local") (`SplineComponent.GetTangentAtDistanceAlongSpline` _spline_2 _returnvalue "Local") (`SplineComponent.GetLocationAtDistanceAlongSpline` _spline _returnvalue_2 "Local") (`SplineComponent.GetTangentAtDistanceAlongSpline` _spline _returnvalue_2 "Local") true))))