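; Test Blueprint whose construction script tiles a static mesh along a spline as spline mesh components.
; Each segment's mesh count and stretched length derive from its length and the mesh's X bounds, with another pass for closed loops.
; GetPositionAndTangentInSpline is meant to supply start/end positions and tangents, but its location and clamped-tangent nodes are unconnected.
; Event graph is empty; a line trace is left unexecuted.
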(fn `UserConstructionScript`
  (locals (SplineMC :type "SplineMeshComponent Object Reference") (MeshIndex :type Integer) (PointIndex :type Integer))
  (bind _pointindex (`local.PointIndex`))
  (bind _spline (`self.Spline`))
  (bind _stetchedmeshlength (`self.StetchedMeshLength`))
  (bind _meshindex (`local.MeshIndex`))
  (bind _currentsplinedistance (`self.CurrentSplineDistance`))
  (bind _spline_2 (`self.Spline`))
  (bind _returnvalue (`SplineComponent.GetDistanceAlongSplineAtSplinePoint` _spline_2 _pointindex))
  (bind _returnvalue_2 (`StaticMesh.GetBoundingBox` (`self.StaticMesh`)))
  (bind (_position _tangent) (`self.GetPositionAndTangentInSpline` _spline _currentsplinedistance _stetchedmeshlength _meshindex))
  (bind (_position_2 _tangent_2) (`self.GetPositionAndTangentInSpline` _spline _currentsplinedistance _stetchedmeshlength (+ _meshindex 1)))
  (set `self.MeshLenght` (- (.x (`.Max` (break `Box` _returnvalue_2))) (.x (break `Box` _returnvalue_2))))
  ; Por cada punto de la spline
  (for _index (range (+ (- (`SplineComponent.GetNumberOfSplinePoints` (`self.Spline`)) 2) 1))
    (set `local.PointIndex` _index :!label _label)
    ; Distancia al punto inicial y longitud del trozo de spline actual
    (set `self.CurrentSplineDistance` _returnvalue)
    (set `self.CurrentSegmentLength` (- (`SplineComponent.GetDistanceAlongSplineAtSplinePoint` _spline_2 (+ _pointindex 1)) _returnvalue))
    (set `self.CurrentSegmentNumMeshes` (/ (`self.CurrentSegmentLength`) (`self.MeshLenght`)))
    ; Si la cantidad de meshes por segmento es mas que 0
    (if (> (`self.CurrentSegmentNumMeshes`) 0)
      ; Tamaño grande
      (bind _output_get (set `self.StetchedMeshLength` (/ (`self.CurrentSegmentLength`) (`self.CurrentSegmentNumMeshes`))))
      ; Si la Mesh estirada es mas pequeña que la mesh original, estira, si no, encoge.
      (if (< (* (`self.MeshLenght`) 1.5) _output_get)
        ; encoger y añadir una mesh
        (set `self.StetchedMeshLength` (/ (`self.CurrentSegmentLength`) (+ (`self.CurrentSegmentNumMeshes`) 1)) :!label _label_2)
        (set `self.CurrentSegmentNumMeshes` (* (`self.CurrentSegmentNumMeshes`) 2)))
      (else
        (goto _label_2)))
    ; Por cantidad de meshes en el actual segmento
    (for _index_2 (range (`self.CurrentSegmentNumMeshes`))
      (set `local.MeshIndex` _index_2)
      ; Creamos el SplineMesh Component con una mesh default
      (bind _returnvalue_3 (`AddComponent|NODE_AddSplineMeshComponent-0`))
      (set `local.SplineMC` _returnvalue_3)
      ; Le seteamos una mesh por variable publica
      (`StaticMeshComponent.SetStaticMesh` (`local.SplineMC`) (`self.StaticMesh`))
      ; Seteamos el forward de la mesh
      (`SplineMeshComponent.SetForwardAxis` (`local.SplineMC`) (`self.In Forward Axis`) true)
      ; Ahijamos el SplineMC a la propia spline. (El blueprint funciona sin esto)
      (`SceneComponent.K2_AttachToComponent` (`local.SplineMC`) (`self.Spline`) "None" "KeepRelative" "KeepRelative" "KeepRelative" true)
      ; Le damos principio y final a la mesh
      (`SplineMeshComponent.SetStartAndEnd` (`local.SplineMC`) _position _tangent _position_2 _tangent_2 true)))
  (if (`SplineComponent.IsClosedLoop` (`self.Spline`))
    (goto _label)))