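; Spline-driven race track actor that builds its road, side walls and finish line in the construction script.
; MakeRoad fits a whole number of stretched spline mesh segments to the spline length, cycling road meshes in repeated runs.
; MakeWalls reuses that segmentation, offsetting walls by half the scaled road width; both follow spline roll and clamp tangents to segment length.
; SetFinishLine places a static mesh at a fractional spline distance plus height offset.
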(fn `MakeRoad`
  (locals (TrackIndex :type Integer) (SplineMeshComp :type "SplineMeshComponent Object Reference"))
  (bind _spline (`self.Spline`))
  (bind _trackindex (`local.TrackIndex`))
  (bind _road_strechedmeshforward (`self.Road_StrechedMeshForward`))
  (bind _splinemeshcomp (`local.SplineMeshComp`))
  (bind _road_originalsize_x (`KismetMathLibrary.BreakVector` (`self.Road_OriginalSize`)))
  (bind _road_originalsize_x_2 (`KismetMathLibrary.BreakVector` (`self.Road_OriginalSize`)))
  (bind _splinemeshcomp_2 (`local.SplineMeshComp`))
  (bind _returnvalue (`KismetMathLibrary.Conv_DoubleToVector2D` (`self.Road_Scale`)))
  (bind (_distance _tangent) (`self.FitSplineMeshAlongSpline` _spline _trackindex _road_strechedmeshforward))
  (bind _returnvalue_roll (`KismetMathLibrary.BreakRotator` (`SplineComponent.GetRotationAtDistanceAlongSpline` (`self.Spline`) (* (`local.TrackIndex`) (`self.Road_StrechedMeshForward`)) "Local")))
  (bind (_returnvalue_min _returnvalue_max) (break `Box` (`StaticMesh.GetBoundingBox` (`|GetArrayItem` (`self.SM_RoadArray`)))))
  (bind (_distance_2 _tangent_2) (`self.FitSplineMeshAlongSpline` _spline (+ _trackindex 1) _road_strechedmeshforward))
  (bind _returnvalue_roll_2 (`KismetMathLibrary.BreakRotator` (`SplineComponent.GetRotationAtDistanceAlongSpline` (`self.Spline`) (* (+ (`local.TrackIndex`) 1) (`self.Road_StrechedMeshForward`)) "Local")))
  ; Mesh sizes
  (set `self.Road_OriginalSize` (- _returnvalue_max _returnvalue_min))
  ; Times for the for Loop
  (bind _output_get (set `self.SplineLenght` (`SplineComponent.GetSplineLength` (`self.Spline`))))
  (set `self.NumOfTracks` (`KismetMathLibrary.FFloor` (/ _output_get _road_originalsize_x_2)))
  ; Rescale mesh size to fit into spline
  (if (> (`self.NumOfTracks`) 0)
    (bind _output_get_2 (set `self.Road_StrechedMeshForward` (/ (`self.SplineLenght`) (`self.NumOfTracks`))))
    (if (< (* _road_originalsize_x 1.5) _output_get_2)
      (bind _output_get_3 (set `self.NumOfTracks` (+ (`self.NumOfTracks`) 1) :!label _label))
      (set `self.Road_StrechedMeshForward` (/ (`self.SplineLenght`) _output_get_3)))
    (else
      (goto _label)))
  (for _index (range (`self.NumOfTracks`))
    (set `local.TrackIndex` _index)
    ; For content
    ;; Create SplineMeshComponent
    (bind _returnvalue_2 (`AddComponent|NODE_AddSplineMeshComponent-0`))
    (set `local.SplineMeshComp` _returnvalue_2)
    ;; Get road type
    (`StaticMeshComponent.SetStaticMesh` (`local.SplineMeshComp`) (`|GetArrayItem` (`self.SM_RoadArray`) (select `int` (mod (/ (`local.TrackIndex`) (`self.RoadTypeTimesRepeated`)) (`KismetArrayLibrary.Array_Length` (`self.SM_RoadArray`))) :`0` 0 :`1` 1 :`2` 2)))
    ;; Simple adjusments
    (`SplineMeshComponent.SetForwardAxis` (`local.SplineMeshComp`) (`self.MeshesForwardAxis`) true)
    (`SceneComponent.K2_AttachToComponent` (`local.SplineMeshComp`) (`self.Spline`) "None" "KeepRelative" "KeepRelative" "KeepRelative" true)
    (`SplineMeshComponent.SetStartScale` _splinemeshcomp_2 _returnvalue true)
    (`SplineMeshComponent.SetEndScale` _splinemeshcomp_2 _returnvalue true)
    (`PrimitiveComponent.SetMaterial` (`local.SplineMeshComp`) 0 (`self.Road_Material`))
    ;; Set start and end position and tangent
    (`SplineMeshComponent.SetStartAndEnd` (`local.SplineMeshComp`) _distance _tangent _distance_2 _tangent_2 true)
    ;; Rotate road
    (`SplineMeshComponent.SetStartRollDegrees` _splinemeshcomp _returnvalue_roll true)
    (`SplineMeshComponent.SetEndRollDegrees` _splinemeshcomp _returnvalue_roll_2 true)
    ;; Collisions
    (`PrimitiveComponent.SetCollisionObjectType` (`local.SplineMeshComp`) (`self.CollisionType`))
    (`PrimitiveComponent.SetCollisionEnabled` (`local.SplineMeshComp`) (`self.CollisionEnable`))))

(fn `MakeWalls`
  (locals (SMC :type "SplineMeshComponent Object Reference") (TrackIndex :type Integer) (WallSide :type Integer))
  (bind _spline (`self.Spline`))
  (bind _road_strechedmeshforward (`self.Road_StrechedMeshForward`))
  (bind _smc (`local.SMC`))
  (bind (_road_originalsize_x _road_originalsize_y) (`KismetMathLibrary.BreakVector` (`self.Road_OriginalSize`)))
  (bind _smc_2 (`local.SMC`))
  (bind _trackindex (`local.TrackIndex`))
  (bind _wallside (`local.WallSide`))
  (bind _returnvalue (`KismetMathLibrary.Conv_DoubleToVector2D` (`self.Wall_Scale`)))
  (bind _returnvalue_roll (`KismetMathLibrary.BreakRotator` (`SplineComponent.GetRotationAtDistanceAlongSpline` (`self.Spline`) (* (`local.TrackIndex`) (`self.Road_StrechedMeshForward`)) "Local")))
  (bind _returnvalue_2 (* _road_originalsize_y (/ (`self.Road_Scale`) 2.0)))
  (bind _returnvalue_roll_2 (`KismetMathLibrary.BreakRotator` (`SplineComponent.GetRotationAtDistanceAlongSpline` (`self.Spline`) (* (+ (`local.TrackIndex`) 1) (`self.Road_StrechedMeshForward`)) "Local")))
  (bind (_distance _tangent) (`self.FitWallsWithRoad` _spline (+ _trackindex 1) _wallside _road_strechedmeshforward _returnvalue_2))
  (bind (_distance_2 _tangent_2) (`self.FitWallsWithRoad` _spline _trackindex _wallside _road_strechedmeshforward _returnvalue_2))
  ; For Track
  (for _index (range (`self.NumOfTracks`))
    (set `local.TrackIndex` _index)
    (for _index_2 (range 2)
      (set `local.WallSide` _index_2)
      ;; Crear SplineMeshComponent
      (bind _returnvalue_3 (`AddComponent|NODE_AddSplineMeshComponent-3`))
      (set `local.SMC` _returnvalue_3)
      ;; Get mesh
      (`StaticMeshComponent.SetStaticMesh` (`local.SMC`) (`self.Walls_Mesh`))
      ;; Simple adjustments
      (`SplineMeshComponent.SetForwardAxis` (`local.SMC`) (`self.MeshesForwardAxis`) true)
      (`SceneComponent.K2_AttachToComponent` (`local.SMC`) (`self.Spline`) "None" "KeepRelative" "KeepRelative" "KeepRelative" true)
      (`SplineMeshComponent.SetStartScale` _smc _returnvalue true)
      (`SplineMeshComponent.SetEndScale` _smc _returnvalue true)
      (`PrimitiveComponent.SetMaterial` (`local.SMC`) 0 (`self.Wall_Material`))
      ;; Set start and end position and tangent
      (`SplineMeshComponent.SetStartAndEnd` (`local.SMC`) _distance_2 _tangent_2 _distance _tangent true)
      ;; Rotate
      (`SplineMeshComponent.SetStartRollDegrees` _smc_2 _returnvalue_roll true)
      (`SplineMeshComponent.SetEndRollDegrees` _smc_2 _returnvalue_roll_2 true)
      ;; Collisions
      (`PrimitiveComponent.SetCollisionObjectType` (`local.SMC`) (`self.CollisionType`))
      (`PrimitiveComponent.SetCollisionEnabled` (`local.SMC`) (`self.CollisionEnable`)))))

(fn `SetFinishLine`
  (locals (SM_Component :type "StaticMeshComponent Object Reference"))
  (bind (_position _rotation) (`self.GetLocationAndRotationAlongSpline` (`self.Spline`) (`self.FL_Location`) (`self.FL_Height`)))
  ; Set Basics
  (bind _returnvalue (`AddComponent|NODE_AddStaticMeshComponent-0`))
  (bind _output_get (set `local.SM_Component` _returnvalue))
  (`StaticMeshComponent.SetStaticMesh` _output_get (`self.FinishLine_SM`))
  (`PrimitiveComponent.SetMaterial` _output_get 0 (`self.FL_Material`))
  ; locate
  (`SceneComponent.K2_SetRelativeLocation` _output_get _position false false)
  (`SceneComponent.K2_SetRelativeRotation` _output_get _rotation false false)
  ; scale
  (`SceneComponent.SetRelativeScale3D` _output_get (`KismetMathLibrary.Conv_DoubleToVector` (`self.FL_Scale`))))

(fn `UserConstructionScript`
  (`self.MakeRoad`)
  (`self.MakeWalls`)
  (`self.SetFinishLine`))