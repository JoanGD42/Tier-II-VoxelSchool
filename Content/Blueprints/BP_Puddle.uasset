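; BP_Puddle is a placeable puddle actor that pairs a ground decal with a Niagara drip effect.
; The construction script passes drop height (Z only) and color to Niagara, applies the same color to the decal, and sets visibility of a cube mesh.
; Two flags toggle particle auto-activation and decal visibility per instance.
; The event graph is empty, and a decal material setter is left unconnected.
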(fn `UserConstructionScript`
  (bind (_dropheight_x _dropheight_y _dropheight_z) (`KismetMathLibrary.BreakVector` (`self.DropHeight`)))
  (bind _niagara (`self.Niagara`))
  (bind _decal (`self.Decal`))
  (bind _niagara_2 (`self.Niagara`))
  (bind _color (`self.Color`))
  (`NiagaraComponent.SetVariableVec3` _niagara_2 "DropHeight" (`KismetMathLibrary.MakeVector` 0.0 0.0 _dropheight_z))
  (`NiagaraComponent.SetNiagaraVariableLinearColor` _niagara_2 "Color" _color)
  (`DecalComponent.SetDecalColor` (`self.Decal`) _color)
  (`SceneComponent.SetVisibility` (`self.Cube`) (`self.CubeVisibility`) false)
  (if (`self.HasParticles`)
    (`ActorComponent.SetAutoActivate` _niagara true)
    (else
      (`ActorComponent.SetAutoActivate` _niagara false)))
  (if (`self.HasPuddle`)
    (`SceneComponent.SetVisibility` _decal true false)
    (else
      (`SceneComponent.SetVisibility` _decal false false))))